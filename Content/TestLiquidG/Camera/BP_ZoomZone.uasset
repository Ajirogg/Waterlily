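; BP_ZoomZone is a level zone that adjusts the camera's terrain zoom while a BP_PawnWithCamera is inside it.
; Begin overlap passes the zone's ZoomModifier to the pawn's AddTerrainZoom, and end overlap passes it to RemoveTerrainZoom.
; The pawn handles the zoom itself.
; Tick checks overlap with the player's controlled pawn but does nothing with the result.
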(event `self.ReceiveActorBeginOverlap`
  (params (OtherActor :type "Actor Object Reference"))
  (bind _asbp_pawn_with_camera (cast `/Game/TestLiquidG/Camera/BP_PawnWithCamera` OtherActor))
  (`/Game/TestLiquidG/Camera/BP_PawnWithCamera.Add Terrain Zoom` _asbp_pawn_with_camera (`self.Zoom Modifier`)))

(event `self.ReceiveActorEndOverlap`
  (params (OtherActor :type "Actor Object Reference"))
  (bind _asbp_pawn_with_camera (cast `/Game/TestLiquidG/Camera/BP_PawnWithCamera` OtherActor))
  (`/Game/TestLiquidG/Camera/BP_PawnWithCamera.Remove Terrain Zoom` _asbp_pawn_with_camera (`self.Zoom Modifier`)))

(event `self.ReceiveTick`
  (params (DeltaSeconds :type "Float (single-precision)"))
  (if (`self.IsOverlappingActor` (`Controller.K2_GetPawn` (`GameplayStatics.GetPlayerController` 0)))
    _))

(fn `UserConstructionScript`)