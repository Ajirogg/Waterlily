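; Base player pawn with a spring-arm camera that switches between water drop and solid forms as temperature crosses solidification or fusion thresholds.
; Form changes spawn and possess a replacement pawn, carrying over health, velocity and temperature, then destroy the old one.
; Health sets mesh scale and mass, with zero triggering game over.
; Camera functions handle yaw, clamped pitch and interpolated zoom from input plus capped terrain zooms, driving arm length, height and FOV.
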(event `TemperatureChanged`
  (params (`new temperature` :type "Float (double-precision)"))
  (bind _is_it__ (`self.isLiquid`))
  (if (and _is_it__ (<= `new temperature` (`self.TemperatureSolidification`)))
    (`self.ChangeForm` "/Game/TestLiquidG/Pawn/BP_SolidState.BP_SolidState_C")
    (else
      (bind _is_it___2 (`self.isSolid`))
      (if (and _is_it___2 (> `new temperature` (`self.TemperatureFusion`)))
        (`self.ChangeForm` "/Game/TestLiquidG/Pawn/Bp_WaterDrop.Bp_WaterDrop_C")))))

(event `InputAction|AfficherViePoids`
  (params (Key :type "Key Structure"))
  (:`Pressed`
    (`KismetSystemLibrary.PrintString` (`KismetStringLibrary.Concat_StrStr` "Vie : " (`KismetStringLibrary.Conv_DoubleToString` (`self.Health`))))
    (`KismetSystemLibrary.PrintString` (`KismetStringLibrary.Concat_StrStr` "Poids : " (`KismetStringLibrary.Conv_DoubleToString` (`self.Poids`))))))

(fn `Add Terrain Zoom`
  (params (`Terrain Zoom` :type "Float (double-precision)"))
  (`KismetArrayLibrary.Array_Add` (`self.Terrain Zooms`) `Terrain Zoom`))

(fn `ApplyZoom`
  (params (`Zoom Input` :type "Float (double-precision)") (DeltaTime :type "Float (double-precision)") (`Max Total Zoom` :type "Float (double-precision)"))
  (locals (TerrainZoomTotal :type "Float (double-precision)" :default 0.0) (ZoomTotal :type "Float (double-precision)") (`Total Zoom Buffer` :type "Float (double-precision)"))
  (bind _springarm (`self.SpringArm`))
  (`|ExecutionSequence`
    (:`then_0`
      ;[1 1 1] Calcul du Zoom Terrain
      (for _array_element (`self.Terrain Zooms`)
        (set `local.TerrainZoomTotal` (+ (`local.TerrainZoomTotal`) _array_element))
        ;[1 1 1] Vérification de la valeur Max
        (bind _asbp_player_camera_manager (cast `/Game/TestLiquidG/Camera/BP_PlayerCameraManager` (`GameplayStatics.GetPlayerCameraManager` 0)))
        (bind _max_terrain_zoom (`/Game/TestLiquidG/Camera/BP_PlayerCameraManager.Max Terrain Zoom` _asbp_player_camera_manager))
        (if (> (`local.TerrainZoomTotal`) _max_terrain_zoom)
          (bind _output_get (set `local.TerrainZoomTotal` _max_terrain_zoom))
          (`KismetSystemLibrary.PrintString` (`KismetStringLibrary.Conv_DoubleToString` _output_get))
          (break))))
    (:`then_1`
      ;[1 1 1] Calcul du Zoom Total
      (bind _output_get_2 (set `local.Total Zoom Buffer` (+ `Zoom Input` (`local.TerrainZoomTotal`) 1.0)))
      (if (not (<= _output_get_2 `Max Total Zoom`))
        (set `local.Total Zoom Buffer` `Max Total Zoom`))
      (if (!= (`self.Target Total Zoom`) (`local.Total Zoom Buffer`))
        (set `self.Target Total Zoom` (`local.Total Zoom Buffer`))
        (set `self.Zoom Lag Current Time` 0.0)))
    (:`then_2`
      ;[1 1 1] Application du Zoom
      (set `self.Zoom Lag Current Time` (+ (`self.Zoom Lag Current Time`) DeltaTime))
      (if (<= (`self.Zoom Lag Current Time`) (`self.Zoom Lag  Max Time`))
        (set `self.Current Total Zoom` (`KismetMathLibrary.FInterpTo` (`self.Current Total Zoom`) (`self.Target Total Zoom`) (/ (`self.Zoom Lag Current Time`) (`self.Zoom Lag  Max Time`)) 1.0))
        (set `SpringArmComponent.TargetArmLength` (* (`self.BaseCameraDistance`) (`self.Current Total Zoom`)) _springarm)
        (set `SpringArmComponent.SocketOffset` (`KismetMathLibrary.MakeVector` 0.0 0.0 (* (`self.BaseCameraHeight`) (`self.Current Total Zoom`))) _springarm)
        (`CameraComponent.SetFieldOfView` (`self.Camera`) (+ (`self.BaseFOV`) (/ (* (`self.BaseFOV`) (`self.Current Total Zoom`)) 10.0)))))))

(fn `Camera Pitch Rotation`
  (params (`Axis Value` :type "Float (double-precision)"))
  (bind _springarm (`self.SpringArm`))
  (set `self.Pitch Angle` (`KismetMathLibrary.FClamp` (+ (`self.Pitch Angle`) `Axis Value`) (`self.Min Pitch Angle`) (`self.Max Pitch Angle`)))
  (`SceneComponent.K2_SetWorldRotation` _springarm (`KismetMathLibrary.MakeRotator` (.roll (`SceneComponent.K2_GetComponentRotation` _springarm)) (`self.Pitch Angle`) (.yaw (`SceneComponent.K2_GetComponentRotation` _springarm))) false false))

(fn `Camera Yaw Rotation`
  (params (`Axis Value` :type "Float (double-precision)"))
  (bind _springarm (`self.SpringArm`))
  (set `self.Yaw Angle` (+ (`self.Yaw Angle`) `Axis Value`))
  (`SceneComponent.K2_SetWorldRotation` _springarm (`KismetMathLibrary.MakeRotator` (.roll (`SceneComponent.K2_GetComponentRotation` _springarm)) (.pitch (`SceneComponent.K2_GetComponentRotation` _springarm)) (`self.Yaw Angle`)) false false))

(fn `ChangeForm`
  (params (Form :type "/Game/TestLiquidG/Camera/BP_PawnWithCamera Class Reference"))
  (locals (OldVelocity :type "Vector Structure"))
  (bind _returnvalue (`self.K2_GetActorLocation`))
  (bind _temperature (`self.GetTemperature` self))
  (bind _output_get (set `local.OldVelocity` (`self.GetVelocity` self)))
  (`self.Get Camera Rotation`)
  (`GameplayStatics.SpawnEmitterAtLocation` "/Game/TestLiquidG/Pawn/P_BounceWall.P_BounceWall" _returnvalue)
  (bind _returnvalue_2 (`|SpawnActorFromClass` Form (`self.GetTransform`) "AlwaysSpawn" "OverrideRootScale" null null))
  (`self.K2_SetActorLocation` _returnvalue_2 _returnvalue false false)
  (set `/Game/TestLiquidG/Camera/BP_PawnWithCamera.Health` (`self.Health`) _returnvalue_2)
  (`self.Scaling` _returnvalue_2)
  (bind _asbp_pawn_with_camera (cast `/Game/TestLiquidG/Camera/BP_PawnWithCamera` _returnvalue_2))
  (bind _asbp_player_controller (cast `/Game/TestLiquidG/Gamemode/BP_PlayerController` (`GameplayStatics.GetPlayerController` 0)))
  (`/Game/TestLiquidG/Gamemode/BP_PlayerController.Possess Pawn` _asbp_player_controller _asbp_pawn_with_camera)
  (`self.K2_DestroyActor`)
  (`PrimitiveComponent.SetPhysicsLinearVelocity` (`/Game/TestLiquidG/Camera/BP_PawnWithCamera.StaticMesh` _returnvalue_2) _output_get false "None")
  (`self.SetTemperature` _returnvalue_2 _temperature))

(fn `Get Camera Infos`
  (returns (`Camera Infos` :type "/Game/TestLiquidG/Camera/CameraInfos Structure"))
  (return (make `/Game/TestLiquidG/Camera/CameraInfos` (`self.Pitch Angle`) (`self.Yaw Angle`))))

(fn `Get Camera Rotation`
  (returns (`Camera Rotation` :type "Rotator Structure"))
  (return (`KismetMathLibrary.MakeRotator` (.roll (`SceneComponent.K2_GetComponentRotation` (`self.Camera`))) (.pitch (`SceneComponent.K2_GetComponentRotation` (`self.Camera`))) (.yaw (`SceneComponent.K2_GetComponentRotation` (`self.SpringArm`))))))

(fn `GetTemperature`
  (returns (Temperature :type "Float (double-precision)"))
  (return (`self.Temperature`)))

(fn `isLiquid`
  (returns (`Is it ?` :type Boolean))
  (return (== (`GameplayStatics.GetObjectClass` self) "/Game/TestLiquidG/Pawn/Bp_WaterDrop.Bp_WaterDrop_C")))

(fn `isSolid`
  (returns (`Is it ?` :type Boolean))
  (return (== (`GameplayStatics.GetObjectClass` self) "/Game/TestLiquidG/Pawn/BP_SolidState.BP_SolidState_C")))

(fn `Remove Terrain Zoom`
  (params (`Terrain Zoom` :type "Float (double-precision)"))
  (for (_array_element _array_index) (`self.Terrain Zooms`)
    (if (== _array_element `Terrain Zoom`)
      (`KismetArrayLibrary.Array_Remove` (`self.Terrain Zooms`) _array_index)
      (break))))

(fn `Scaling`
  (bind _staticmesh (`self.StaticMesh`))
  (bind _assettings (cast `/Game/TestLiquidG/Pawn/Settings` (`GameplayStatics.GetGameInstance`)))
  (bind _returnvalue (* (/ (`self.Health`) 10.0) (`/Game/TestLiquidG/Pawn/Settings.BallScale` _assettings)))
  (`SceneComponent.SetRelativeScale3D` _staticmesh (`KismetMathLibrary.MakeVector` _returnvalue _returnvalue _returnvalue))
  (`KismetSystemLibrary.PrintString` (`KismetStringLibrary.Concat_StrStr` "Scale  :  " (`KismetStringLibrary.Conv_DoubleToString` _returnvalue)))
  (bind _returnvalue_2 (* _returnvalue 20.0))
  (set `self.Poids` _returnvalue_2)
  (`PrimitiveComponent.SetMassOverrideInKg` _staticmesh "None" _returnvalue_2 true)
  (`KismetSystemLibrary.PrintString` (`KismetStringLibrary.Concat_StrStr` "Mass  :  " (`KismetStringLibrary.Conv_DoubleToString` _returnvalue_2)))
  (if (== (`self.Health`) 0.0)
    (`self.K2_DestroyActor`)
    (bind _returnvalue_3 (`|CreateWidget` "/Game/UI/BP_GameOver.BP_GameOver_C" (`GameplayStatics.GetPlayerController` 0)))
    (`UserWidget.AddToViewport` _returnvalue_3 0)))

(fn `Set Camera Infos`
  (params (`Camera Infos` :type "/Game/TestLiquidG/Camera/CameraInfos Structure"))
  (bind (_ptichangle _yawangle) (break `/Game/TestLiquidG/Camera/CameraInfos` `Camera Infos`))
  (`self.Set Enable Camera Rotation Lag` false)
  (set `self.Pitch Angle` _ptichangle)
  (set `self.Yaw Angle` _yawangle)
  (`self.Camera Yaw Rotation` 0.0)
  (`self.Camera Pitch Rotation` 0.0)
  (`self.Set Enable Camera Rotation Lag` true))

(fn `Set Camera Rotation`
  (params (`Camera Rotator` :type "Rotator Structure"))
  (`SceneComponent.K2_SetWorldRotation` (`self.SpringArm`) (`KismetMathLibrary.MakeRotator` 0.0 (.pitch `Camera Rotator`) (.yaw `Camera Rotator`)) false false))

(fn `Set Enable Camera Lag`
  (params (`Enable Camera Lag` :type Boolean))
  (set `SpringArmComponent.bEnableCameraLag` `Enable Camera Lag` (`self.SpringArm`)))

(fn `Set Enable Camera Rotation Lag`
  (params (`Enable Camera Rotation Lag` :type Boolean))
  (bind _springarm (`self.SpringArm`))
  (set `SpringArmComponent.bEnableCameraRotationLag` `Enable Camera Rotation Lag` _springarm)
  (set `SpringArmComponent.CameraRotationLagSpeed` 0.0 _springarm))

(fn `SetTemperature`
  (params (new :type "Float (double-precision)"))
  (returns (temperature :type "Float (double-precision)"))
  (bind _output_get (set `self.Temperature` (`KismetMathLibrary.FClamp` new 0.0 200.0)))
  (`self.TemperatureChanged` _output_get)
  (`KismetSystemLibrary.PrintString` (`KismetStringLibrary.Concat_StrStr` "Température :" (`KismetStringLibrary.Conv_DoubleToString` _output_get)))
  (return _output_get))

(fn `UserConstructionScript`)