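; Player camera manager that drives zoom and rotation on BP_PawnWithCamera pawns and tracks the pawn being looked at.
; Each tick it applies clamped input zoom, then line-traces from the camera to update the selected pawn, though custom-depth highlighting is only ever set false.
; UnlockCamera flip-flops on press and release to gate pitch; yaw is always applied.
; Line-of-sight zoom limiting exists but is never called, so max zoom stays constant.
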(event `Init Max Total Zoom`
  ;[1 1 1] Collision Camera
  (bind _output_get (set `self.Base Max Total Zoom` (+ (`self.Max Input Zoom`) (`self.Max Terrain Zoom`) 1.0)))
  (set `self.Max Total Zoom` _output_get))

(event `self.ReceiveTick`
  (params (DeltaSeconds :type "Float (single-precision)"))
  ;[1 1 1] Event Tick
  (`|ExecutionSequence`
    (:`then_1`
      ;[1 1 1] Application du Zoom
      (bind _asbp_pawn_with_camera (cast `/Game/TestLiquidG/Camera/BP_PawnWithCamera` (`GameplayStatics.GetPlayerPawn` 0)))
      (`/Game/TestLiquidG/Camera/BP_PawnWithCamera.ApplyZoom` _asbp_pawn_with_camera (`self.Input Zoom`) DeltaSeconds (`self.Max Total Zoom`)))
    (:`then_2`
      ;[1 1 1] Pawn Selection
      (`self.Find and Highlight Selected Pawn`))))

(event `EstimateMaxCameraZoom`
  ;[1 1 1] Collision Camera
  (bind (_isblocked _hit_distance_from_pawn) (`self.IsLineOfSightBlocked`))
  (if _isblocked
    (bind _appropriate_zoom (`self.Find Appropriate Zoom` _hit_distance_from_pawn))
    (set `self.Max Total Zoom` _appropriate_zoom)
    (else
      (set `self.Max Total Zoom` (`self.Base Max Total Zoom`)))))

(event `self.ReceiveBeginPlay`
  ;[1 1 1] Event BeginPlay
  (`self.Init Max Total Zoom`))

(event `InputAction|ZoomIn`
  (params (Key :type "Key Structure"))
  ;[1 1 1] Input du Zoom
  (:`Pressed`
    (set `self.Input Zoom` (+ (`self.Input Zoom`) (* -1.0 (`self.Input Zoom Increment`))))
    (if (< (`self.Input Zoom`) 0.0)
      (set `self.Input Zoom` 0.0))))

(event `InputAction|ZoomOut`
  (params (Key :type "Key Structure"))
  ;[1 1 1] Input du Zoom
  (:`Pressed`
    (set `self.Input Zoom` (+ (`self.Input Zoom`) (* 1.0 (`self.Input Zoom Increment`))))
    (if (> (`self.Input Zoom`) (`self.Max Input Zoom`))
      (set `self.Input Zoom` (`self.Max Input Zoom`)))))

(event `InputAction|UnlockCamera`
  (params (Key :type "Key Structure"))
  ;[1 1 1] Yaw Rotation Input
  (:`Pressed`
    (bind _isa (`/Engine/EditorBlueprintResources/StandardMacros.FlipFlop` :!label _label)
      (:`A`
        _)
      (:`B`
        _))
    (set `self.Is Yaw Rotation Unlock` _isa))
  (:`Released`
    (goto _label)))

(event `InputAxis|YawRotation`
  (params (AxisValue :type "Float (single-precision)"))
  ;[1 1 1] Yaw Rotation Input
  (if true
    (bind _asbp_pawn_with_camera (cast `/Game/TestLiquidG/Camera/BP_PawnWithCamera` (`Controller.K2_GetPawn` (`GameplayStatics.GetPlayerController` 0))))
    (`/Game/TestLiquidG/Camera/BP_PawnWithCamera.Camera Yaw Rotation` _asbp_pawn_with_camera AxisValue)))

(event `InputAction|UnlockCamera`
  (params (Key :type "Key Structure"))
  ;[1 1 1] Pitch Rotation Input
  (:`Pressed`
    (bind _isa (`/Engine/EditorBlueprintResources/StandardMacros.FlipFlop` :!label _label_2)
      (:`A`
        _)
      (:`B`
        _))
    (set `self.Is Pitch Rotation Unlock` _isa))
  (:`Released`
    (goto _label_2)))

(event `InputAxis|Pitch Rotation`
  (params (AxisValue :type "Float (single-precision)"))
  ;[1 1 1] Pitch Rotation Input
  (if (`self.Is Pitch Rotation Unlock`)
    (bind _asbp_pawn_with_camera (cast `/Game/TestLiquidG/Camera/BP_PawnWithCamera` (`Controller.K2_GetPawn` (`GameplayStatics.GetPlayerController` 0))))
    (`/Game/TestLiquidG/Camera/BP_PawnWithCamera.Camera Pitch Rotation` _asbp_pawn_with_camera AxisValue)))

(fn `Find and Highlight Selected Pawn`
  (bind _current_drawn_pawn (`self.Current Drawn Pawn`))
  (bind _current_drawn_pawn_2 (`self.Current Drawn Pawn`))
  (bind _asbp_pawn_with_camera (cast `/Game/TestLiquidG/Camera/BP_PawnWithCamera` (`Controller.K2_GetPawn` (`GameplayStatics.GetPlayerController` 0))))
  (bind _returnvalue (`SceneComponent.K2_GetComponentLocation` (`/Game/TestLiquidG/Camera/BP_PawnWithCamera.Camera` _asbp_pawn_with_camera)))
  (bind (_outhit _returnvalue_2) (`KismetSystemLibrary.LineTraceSingle` _returnvalue (+ _returnvalue (* (`KismetMathLibrary.GreaterGreater_VectorRotator` (`KismetMathLibrary.MakeVector` 1.0) (`KismetMathLibrary.MakeRotator` 0.0 (.pitch (`SceneComponent.K2_GetComponentRotation` (`/Game/TestLiquidG/Camera/BP_PawnWithCamera.Camera` _asbp_pawn_with_camera))) (.yaw (`SceneComponent.K2_GetComponentRotation` (`/Game/TestLiquidG/Camera/BP_PawnWithCamera.Camera` _asbp_pawn_with_camera))))) 10000.0)) "TraceTypeQuery1"))
  (if _returnvalue_2
    (bind _asbp_pawn_with_camera_2 (cast `/Game/TestLiquidG/Camera/BP_PawnWithCamera` (`.HitActor` (`GameplayStatics.BreakHitResult` _outhit)))
      (:`then`
        (if (!= _asbp_pawn_with_camera_2 (`self.Current Drawn Pawn`))
          (if (`KismetSystemLibrary.IsValid` _current_drawn_pawn_2)
            (`PrimitiveComponent.SetRenderCustomDepth` (`/Game/TestLiquidG/Camera/BP_PawnWithCamera.StaticMesh` _current_drawn_pawn_2) false))
          (bind _output_get (set `self.Current Drawn Pawn` _asbp_pawn_with_camera_2))
          (`PrimitiveComponent.SetRenderCustomDepth` (`/Game/TestLiquidG/Camera/BP_PawnWithCamera.StaticMesh` _output_get) false)
          (`KismetSystemLibrary.PrintString` "Outinling!")))
      (:`CastFailed`
        (if (`KismetSystemLibrary.IsValid` _current_drawn_pawn) :!label _label
          (`PrimitiveComponent.SetRenderCustomDepth` (`/Game/TestLiquidG/Camera/BP_PawnWithCamera.StaticMesh` _current_drawn_pawn) false)
          (set `self.Current Drawn Pawn` null))))
    (else
      (goto _label))))

(fn `Find Appropriate Zoom`
  (params (`Distance Pawn to Collision` :type "Float (double-precision)"))
  (returns (`Appropriate Zoom` :type "Float (double-precision)"))
  (locals (Zoom :type "Float (double-precision)") (`Camera Location` :type "Vector Structure"))
  (set `local.Zoom` (`self.Base Max Total Zoom`))
  (bind _asbp_pawn_with_camera (cast `/Game/TestLiquidG/Camera/BP_PawnWithCamera` (`Controller.K2_GetPawn` (`GameplayStatics.GetPlayerController` 0))))
  (bind _springarm (`/Game/TestLiquidG/Camera/BP_PawnWithCamera.SpringArm` _asbp_pawn_with_camera))
  (bind _output_get (set `local.Camera Location` (`KismetMathLibrary.MakeVector` (`SpringArmComponent.TargetArmLength` _springarm) 0.0 (.z (`SpringArmComponent.SocketOffset` _springarm)))))
  (while (> (* (`KismetMathLibrary.VSize` _output_get) (`local.Zoom`)) `Distance Pawn to Collision`)
    (set `local.Zoom` (- (`local.Zoom`) (`self.Input Zoom Increment`))))
  (return (`local.Zoom`)))

(fn `Get Selected Pawn`
  (returns (`Selected Pawn` :type "/Game/TestLiquidG/Camera/BP_PawnWithCamera Object Reference"))
  (return (`self.Current Drawn Pawn`)))

(fn `Is A Pawn Selected`
  (returns (selected :type Boolean))
  (return (`KismetSystemLibrary.IsValid` (`self.Current Drawn Pawn`))))

(fn `IsLineOfSightBlocked`
  (returns (IsBlocked :type Boolean) (`Hit Distance From Pawn` :type "Float (double-precision)"))
  (bind _asbp_pawn_with_camera (cast `/Game/TestLiquidG/Camera/BP_PawnWithCamera` (`Controller.K2_GetPawn` (`GameplayStatics.GetPlayerController` 0))))
  (bind _springarm (`/Game/TestLiquidG/Camera/BP_PawnWithCamera.SpringArm` _asbp_pawn_with_camera))
  (bind _outhit (`KismetSystemLibrary.LineTraceSingle` :`Start` (+ (`KismetMathLibrary.GreaterGreater_VectorRotator` (`KismetMathLibrary.MakeVector` (`SpringArmComponent.TargetArmLength` _springarm) 0.0 (.z (`SpringArmComponent.SocketOffset` _springarm))) (`SceneComponent.RelativeRotation` _springarm)) (`SceneComponent.K2_GetComponentLocation` _springarm)) :`End` (`SceneComponent.K2_GetComponentLocation` (`/Game/TestLiquidG/Camera/BP_PawnWithCamera.StaticMesh` _asbp_pawn_with_camera)) :`TraceChannel` "TraceTypeQuery1" :`DrawDebugType` "ForOneFrame" :`bIgnoreSelf` false))
  (bind (_bblockinghit _binitialoverlap _time _distance _location _impactpoint _normal _impactnormal _physmat _hitactor) (`GameplayStatics.BreakHitResult` _outhit))
  (`KismetSystemLibrary.PrintString` (`KismetStringLibrary.Conv_DoubleToString` (`KismetMathLibrary.VSize` _location)))
  (return (!= _hitactor _asbp_pawn_with_camera) (`KismetMathLibrary.VSize` (- (`SceneComponent.K2_GetComponentLocation` (`/Game/TestLiquidG/Camera/BP_PawnWithCamera.StaticMesh` _asbp_pawn_with_camera)) _location))))

(fn `UserConstructionScript`)