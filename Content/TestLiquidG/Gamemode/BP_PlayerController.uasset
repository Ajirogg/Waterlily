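; BP_PlayerController is a player controller that lets the player switch to the selected pawn by pressing R.
; It gets the selection from BP_PlayerCameraManager and prints a message when nothing is selected.
; PossessPawn copies camera infos from the current BP_PawnWithCamera to the target before unpossessing and possessing, so camera settings carry over.
; Invalid targets or incompatible current pawns only print an error.
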(event `Key|R`
  (params (Key :type "Key Structure"))
  (:`Pressed`
    (bind _asbp_player_camera_manager (cast `/Game/TestLiquidG/Camera/BP_PlayerCameraManager` (`GameplayStatics.GetPlayerCameraManager` 0)))
    (bind _selected (`/Game/TestLiquidG/Camera/BP_PlayerCameraManager.Is A Pawn Selected` _asbp_player_camera_manager))
    (if _selected
      (bind _selected_pawn (`/Game/TestLiquidG/Camera/BP_PlayerCameraManager.Get Selected Pawn` _asbp_player_camera_manager))
      (`self.Possess Pawn` _selected_pawn)
      (else
        (`KismetSystemLibrary.PrintText` "Aucune Pawn séléctionnée")))))

(event `InputAction|MenuPause`
  (params (Key :type "Key Structure")))

(fn `Possess Pawn`
  (params (`Pawn To Possess` :type "/Game/TestLiquidG/Camera/BP_PawnWithCamera Object Reference"))
  (if (`KismetSystemLibrary.IsValid` `Pawn To Possess`)
    (bind _asbp_pawn_with_camera (cast `/Game/TestLiquidG/Camera/BP_PawnWithCamera` (`self.K2_GetPawn`))
      (:`then`
        (bind _camera_infos (`/Game/TestLiquidG/Camera/BP_PawnWithCamera.Get Camera Infos` _asbp_pawn_with_camera))
        (`self.UnPossess`)
        (`/Game/TestLiquidG/Camera/BP_PawnWithCamera.Set Camera Infos` `Pawn To Possess` _camera_infos)
        (`self.Possess` `Pawn To Possess`))
      (:`CastFailed`
        (`KismetSystemLibrary.PrintString` "Current Possessed Pawn is incompatible with \"Possess Pawn\"")))
    (else
      (`KismetSystemLibrary.PrintString` "Pawn To Possess is invalid"))))

(fn `UserConstructionScript`)