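; BP_Trigger is a trigger actor that counts down a limited absorption capacity while a water drop overlaps it.
; Box overlap events with Bp_WaterDrop set and clear a single overlap flag.
; Tick feeds a one-second Delay, so each second of overlap decrements NbGoutte and calls Absorber.
; The actor destroys itself once NbGoutte runs out, or on an overlapping check when it is already empty.
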(event `self.ReceiveTick`
  (params (DeltaSeconds :type "Float (single-precision)"))
  (bind _nbgoutte (`self.nbGoutte`))
  (bind _returnvalue (> _nbgoutte 0))
  (`KismetSystemLibrary.Delay` (+ 0.0 1.0))
  (if (`self.Overlaping`)
    (if _returnvalue
      (set `self.nbGoutte` (- _nbgoutte 1))
      (`self.Absorber`)
      (if (not _returnvalue)
        (`self.K2_DestroyActor` :!label _label))
      (else
        (goto _label)))))

(event `self.Box.OnComponentBeginOverlap`
  (params (OverlappedComponent :type "PrimitiveComponent Object Reference") (OtherActor :type "Actor Object Reference") (OtherComp :type "PrimitiveComponent Object Reference") (OtherBodyIndex :type Integer) (bFromSweep :type Boolean) (SweepResult :type "HitResult Structure (by ref)"))
  (cast `/Game/TestLiquidG/Pawn/Bp_WaterDrop` OtherActor)
  (set `self.Overlaping` true))

(event `self.Box.OnComponentEndOverlap`
  (params (OverlappedComponent :type "PrimitiveComponent Object Reference") (OtherActor :type "Actor Object Reference") (OtherComp :type "PrimitiveComponent Object Reference") (OtherBodyIndex :type Integer))
  (cast `/Game/TestLiquidG/Pawn/Bp_WaterDrop` OtherActor)
  (set `self.Overlaping` false))

(fn `UserConstructionScript`)