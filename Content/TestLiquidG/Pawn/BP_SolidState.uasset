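; Player pawn for the solid state, a physics mesh that can switch into a water drop.
; Camera-yaw-relative input becomes torque when Rotation is set, otherwise force applied only while grounded and under the XY speed cap.
; Hit events maintain grounding through a retriggerable delay, and both movement branches feed a delayed Temperature increase.
; ChangerEtat spawns Bp_WaterDrop with the current Health, possesses it and destroys this pawn.
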(event `InputAxis|AvancerReculer`
  (params (AxisValue :type "Float (single-precision)"))
  (`self.AddMovementInput` (`KismetMathLibrary.GetForwardVector` (`KismetMathLibrary.MakeRotator` (.roll (`SceneComponent.K2_GetComponentRotation` (`self.Camera`))) 0.0 (.yaw (`SceneComponent.K2_GetComponentRotation` (`self.Camera`))))) AxisValue))

(event `InputAxis|DroiteGauche`
  (params (AxisValue :type "Float (single-precision)"))
  (`self.AddMovementInput` (`KismetMathLibrary.GetRightVector` (`KismetMathLibrary.MakeRotator` (.roll (`SceneComponent.K2_GetComponentRotation` (`self.Camera`))) 0.0 (.yaw (`SceneComponent.K2_GetComponentRotation` (`self.Camera`))))) AxisValue))

(event `self.ReceiveTick`
  (params (DeltaSeconds :type "Float (single-precision)"))
  (bind _returnvalue (`self.ConsumeMovementInputVector`))
  (if (`self.Rotation`)
    (bind _returnvalue_2 (`KismetMathLibrary.Normal` _returnvalue))
    (bind _returnvalue_3 (* (* _returnvalue_2 (`self.RotationForce`)) DeltaSeconds))
    (`PrimitiveComponent.AddTorqueInDegrees` (`self.StaticMesh`) _returnvalue_3 "None" true)
    (`KismetSystemLibrary.PrintString` (`KismetStringLibrary.Conv_VectorToString` _returnvalue_3))
    (`KismetSystemLibrary.Delay` 0.25 :!label _label)
    (`self.SetTemperature` (+ (`self.Temperature`) 2.5))
    (elif (`self.IsGrounded`)
      (bind _over_speed (`self.isOverspeed` (`self.VelocityMax`)))
      (if (not _over_speed)
        (`PrimitiveComponent.AddForce` (`self.StaticMesh`) (* (* _returnvalue_2 (`self.LinearForce`)) DeltaSeconds) "None" true)
        (goto _label)))))

(event `InputAction|ChangerEtat`
  (params (Key :type "Key Structure"))
  (bind _returnvalue (`self.K2_GetActorLocation`))
  (:`Pressed`
    (`GameplayStatics.SpawnEmitterAtLocation` "/Game/TestLiquidG/Pawn/P_BounceWall.P_BounceWall" _returnvalue)
    (bind _returnvalue_2 (`|SpawnActorFromClass` "/Game/TestLiquidG/Pawn/Bp_WaterDrop.Bp_WaterDrop_C" (`self.GetTransform`) "AlwaysSpawn" "OverrideRootScale" null null))
    (set `/Game/TestLiquidG/Camera/BP_PawnWithCamera.Health` (`self.Health`) _returnvalue_2)
    (`self.Scaling` _returnvalue_2)
    (`self.K2_SetActorLocation` _returnvalue_2 _returnvalue false false)
    (bind _asbp_player_controller (cast `/Game/TestLiquidG/Gamemode/BP_PlayerController` (`GameplayStatics.GetPlayerController` 0)))
    (`/Game/TestLiquidG/Gamemode/BP_PlayerController.Possess Pawn` _asbp_player_controller _returnvalue_2)
    (`self.K2_DestroyActor`)))

(event `self.StaticMesh.OnComponentHit`
  (params (HitComponent :type "PrimitiveComponent Object Reference") (OtherActor :type "Actor Object Reference") (OtherComp :type "PrimitiveComponent Object Reference") (NormalImpulse :type "Vector Structure") (Hit :type "HitResult Structure (by ref)"))
  (set `self.IsGrounded` true)
  (`KismetSystemLibrary.RetriggerableDelay` 0.1)
  (set `self.IsGrounded` false))

(fn `isOverspeed`
  (params (maxVelocity :type "Float (double-precision)"))
  (returns (`Over speed` :type Boolean))
  (return (>= (`KismetMathLibrary.VSizeXY` (`self.GetVelocity` self)) maxVelocity)))

(fn `UserConstructionScript`)