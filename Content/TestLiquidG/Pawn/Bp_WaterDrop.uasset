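; Bp_WaterDrop is a water drop pawn that can split, merge with other drops and trigger a state change through a temperature call.
; Camera-relative input becomes a physics force on the mesh each Tick, with an upward bias and scaling by speed and weight.
; Splitting halves Health and spawns a sibling drop with the same amount.
; When the controlled drop overlaps another, it absorbs its Health, destroys it and rescales.
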(event `self.ReceiveBeginPlay`
  (`self.Scaling`))

(event `InputAction|Séparer`
  (params (Key :type "Key Structure"))
  (bind _returnvalue (`self.GetTransform`))
  ;[1 1 1] Séparation
  (:`Pressed`
    (if (<= 1.0 (`self.Health`))
      (bind _output_get (set `self.Health` (/ (`self.Health`) 2.0)))
      (`self.Scaling`)
      (bind _returnvalue_2 (`|SpawnActorFromClass` "Bp_WaterDrop_C" (`KismetMathLibrary.MakeTransform` (`KismetMathLibrary.MakeVector` (+ (.x (.location _returnvalue)) 10.0) (.y (.location _returnvalue)) (.z (.location _returnvalue))) (.rotation _returnvalue) (.scale _returnvalue)) "AlwaysSpawn" "OverrideRootScale" null null))
      (set `/Game/TestLiquidG/Camera/BP_PawnWithCamera.Health` _output_get _returnvalue_2)
      (`self.Scaling` _returnvalue_2))))

(event `InputAction|ChangerEtat`
  (params (Key :type "Key Structure"))
  ;[1 1 1] Changement état
  (:`Pressed`
    (`self.SetTemperature` 30.0)))

(event `InputAxis|AvancerReculer`
  (params (AxisValue :type "Float (single-precision)"))
  ;[1 1 1] Déplacement
  (`self.AddMovementInput` (`KismetMathLibrary.GetForwardVector` (`KismetMathLibrary.MakeRotator` (.roll (`SceneComponent.K2_GetComponentRotation` (`self.Camera`))) 0.0 (.yaw (`SceneComponent.K2_GetComponentRotation` (`self.Camera`))))) AxisValue))

(event `InputAxis|DroiteGauche`
  (params (AxisValue :type "Float (single-precision)"))
  ;[1 1 1] Déplacement
  (`self.AddMovementInput` (`KismetMathLibrary.GetRightVector` (`KismetMathLibrary.MakeRotator` (.roll (`SceneComponent.K2_GetComponentRotation` (`self.Camera`))) 0.0 (.yaw (`SceneComponent.K2_GetComponentRotation` (`self.Camera`))))) AxisValue))

(event `self.ReceiveTick`
  (params (DeltaSeconds :type "Float (single-precision)"))
  ;[1 1 1] Déplacement
  (bind _returnvalue (`self.ConsumeMovementInputVector`))
  (`PrimitiveComponent.AddForce` (`self.StaticMesh`) (* (* (+ _returnvalue (0.0 0.0 3.0)) (`self.SpeedMultiplicater`)) (* (`self.Poids`) 1.5)) "None" false))

(event `self.Sphere.OnComponentBeginOverlap`
  (params (OverlappedComponent :type "PrimitiveComponent Object Reference") (OtherActor :type "Actor Object Reference") (OtherComp :type "PrimitiveComponent Object Reference") (OtherBodyIndex :type Integer) (bFromSweep :type Boolean) (SweepResult :type "HitResult Structure (by ref)"))
  (bind _returnvalue (`Controller.K2_GetPawn` (`GameplayStatics.GetPlayerController` 0)))
  (bind _asbp_water_drop (cast `/Game/TestLiquidG/Pawn/Bp_WaterDrop` OtherActor))
  (if (and (== self _returnvalue) (!= _returnvalue _asbp_water_drop))
    (set `self.Health` (+ (`self.Health`) (`/Game/TestLiquidG/Camera/BP_PawnWithCamera.Health` _asbp_water_drop)))
    (`self.K2_DestroyActor` _asbp_water_drop)
    (`self.Scaling`)))

(fn `UserConstructionScript`)