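; BP_Pawn is a test pawn that turns player axis input into physics spin on a Sphere component.
; AvancerReculer and DroiteGauche add movement input along Camera1's forward and right vectors.
; Tick consumes that vector, scales it by delta time and sets it directly as the sphere's angular velocity in degrees, replacing the current spin rather than adding to it.
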(event `InputAxis|AvancerReculer`
  (params (AxisValue :type "Float (single-precision)"))
  (`self.AddMovementInput` (`SceneComponent.GetForwardVector` (`self.Camera1`)) AxisValue))

(event `InputAxis|DroiteGauche`
  (params (AxisValue :type "Float (single-precision)"))
  (`self.AddMovementInput` (`SceneComponent.GetRightVector` (`self.Camera1`)) AxisValue))

(event `self.ReceiveTick`
  (params (DeltaSeconds :type "Float (single-precision)"))
  (bind _returnvalue (`self.ConsumeMovementInputVector`))
  (`PrimitiveComponent.SetPhysicsAngularVelocityInDegrees` (`self.Sphere`) (* _returnvalue (`KismetMathLibrary.Conv_DoubleToVector` DeltaSeconds)) false "None"))

(fn `UserConstructionScript`)