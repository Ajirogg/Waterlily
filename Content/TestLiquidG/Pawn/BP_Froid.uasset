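; BP_Froid is a trigger volume that repeatedly calls Froid (French for "cold") while the camera pawn is inside it.
; Box begin and end overlap events cast the other actor to BP_PawnWithCamera and set or clear an Overlap flag.
; Tick runs through a Delay, throttling the flag check and resulting call to roughly four times per second.
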(event `self.ReceiveTick`
  (params (DeltaSeconds :type "Float (single-precision)"))
  (`KismetSystemLibrary.Delay` 0.25)
  (if (`self.overlap`)
    (`self.Froid`)))

(event `self.Box.OnComponentBeginOverlap`
  (params (OverlappedComponent :type "PrimitiveComponent Object Reference") (OtherActor :type "Actor Object Reference") (OtherComp :type "PrimitiveComponent Object Reference") (OtherBodyIndex :type Integer) (bFromSweep :type Boolean) (SweepResult :type "HitResult Structure (by ref)"))
  (cast `/Game/TestLiquidG/Camera/BP_PawnWithCamera` OtherActor)
  (set `self.overlap` true))

(event `self.Box.OnComponentEndOverlap`
  (params (OverlappedComponent :type "PrimitiveComponent Object Reference") (OtherActor :type "Actor Object Reference") (OtherComp :type "PrimitiveComponent Object Reference") (OtherBodyIndex :type Integer))
  (cast `/Game/TestLiquidG/Camera/BP_PawnWithCamera` OtherActor)
  (set `self.overlap` false))

(fn `UserConstructionScript`)