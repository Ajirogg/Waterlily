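; BP_Character is a test pawn that drives a physics sphere from camera-relative movement input.
; The AvancerReculer and DroiteGauche axes add movement input along Camera1's forward and right vectors.
; Tick consumes that vector, multiplies it by delta seconds and sets it directly as the Sphere's angular velocity in degrees, replacing the current spin.
; The input direction therefore serves as the rotation axis.
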(event `InputAxis|AvancerReculer`
  (params (AxisValue :type "Float (single-precision)"))
  (`self.AddMovementInput` (`SceneComponent.GetForwardVector` (`self.Camera1`)) AxisValue))

(event `InputAxis|DroiteGauche`
  (params (AxisValue :type "Float (single-precision)"))
  (`self.AddMovementInput` (`SceneComponent.GetRightVector` (`self.Camera1`)) AxisValue))

(event `self.ReceiveTick`
  (params (DeltaSeconds :type "Float (single-precision)"))
  (bind _returnvalue (`self.ConsumeMovementInputVector`))
  (`PrimitiveComponent.SetAllPhysicsAngularVelocityInDegrees` (`self.sphere`) (* _returnvalue (`KismetMathLibrary.Conv_DoubleToVector` DeltaSeconds)) false))

(fn `UserConstructionScript`)