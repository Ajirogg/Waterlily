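; BP_Salir is an exit trigger ("salir") that signals when the water drop or solid-state actor is inside its box.
; Box begin and end overlap events set and clear an Overlap flag for Bp_WaterDrop or BP_SolidState actors.
; Tick runs through a quarter-second Delay, so it calls Salir repeatedly at that interval while the flag is set.
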(event `self.ReceiveTick`
  (params (DeltaSeconds :type "Float (single-precision)"))
  (`KismetSystemLibrary.Delay` 0.25)
  (if (`self.overlap`)
    (`self.Salir`)))

(event `self.Box.OnComponentBeginOverlap`
  (params (OverlappedComponent :type "PrimitiveComponent Object Reference") (OtherActor :type "Actor Object Reference") (OtherComp :type "PrimitiveComponent Object Reference") (OtherBodyIndex :type Integer) (bFromSweep :type Boolean) (SweepResult :type "HitResult Structure (by ref)"))
  (cast `/Game/TestLiquidG/Pawn/Bp_WaterDrop` OtherActor
    (:`then`
      _)
    (:`CastFailed`
      (cast `/Game/TestLiquidG/Pawn/BP_SolidState` OtherActor)))
  (set `self.overlap` true))

(event `self.Box.OnComponentEndOverlap`
  (params (OverlappedComponent :type "PrimitiveComponent Object Reference") (OtherActor :type "Actor Object Reference") (OtherComp :type "PrimitiveComponent Object Reference") (OtherBodyIndex :type Integer))
  (cast `/Game/TestLiquidG/Pawn/Bp_WaterDrop` OtherActor
    (:`then`
      _)
    (:`CastFailed`
      (cast `/Game/TestLiquidG/Pawn/BP_SolidState` OtherActor)))
  (set `self.overlap` false))

(fn `UserConstructionScript`)